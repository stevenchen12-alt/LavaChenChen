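; BP_ExplodeFloor is an explosion actor that blows apart nearby objects tagged "Explode" when StartExplosion is called.
; A sphere trace finds them, then enables physics on skeletal meshes below a target bone, static mesh actors and push-button frames.
; Both mesh types get upward and random angular impulses plus a timed lifespan.
; A RadialForce impulse fires afterward, while geometry collection fracture nodes remain unconnected.
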(event Custom|StartExplosion
  (bind _outhits (Collision|MultiSphereTraceByChannel (Transformation|GetActorLocation) (Transformation|GetActorLocation) 1e+03 "TraceTypeQuery1" false 0 "None"))
  (for _array_element _outhits
    (if (Actor|ActorHasTag (.HitActor (Collision|BreakHitResult _array_element)) "Explode")
      (Utilities|FlowControl|Sequence
        (:then_0
          (bind _asskeletal_mesh_component (Utilities|Casting|CastToSkeletalMeshComponent (.HitComponent (Collision|BreakHitResult _array_element))))
          (Class|SkeletalMeshComponent|SetAllBodiesBelowSimulatePhysics _asskeletal_mesh_component (Variables|Default|GetTargetBone) true false)
          (Class|PrimitiveComponent|WakeRigidBody _asskeletal_mesh_component "None")
          (Physics|AddImpulse _asskeletal_mesh_component "0.000000,0.000000,500.000000" "None" true)
          (Class|PrimitiveComponent|AddAngularImpulseinDegrees _asskeletal_mesh_component (Math|Conversions|ToVector(Float) (Math|Random|RandomFloatinRange -1.8e+02 1.8e+02)) "None" true)
          (Actor|SetLifeSpan (.HitActor (Collision|BreakHitResult _array_element)) 1e+01))
        (:then_1
          (bind _asstatic_mesh_actor (Utilities|Casting|CastToStaticMeshActor (.HitActor (Collision|BreakHitResult _array_element)))
            (:then
              (Physics|SetSimulatePhysics (Variables|/Script/Engine.StaticMeshActor|GetStaticMeshComponent _asstatic_mesh_actor) true)
              (Class|PrimitiveComponent|WakeRigidBody (Variables|/Script/Engine.StaticMeshActor|GetStaticMeshComponent _asstatic_mesh_actor) "None")
              (Physics|AddImpulse (Variables|/Script/Engine.StaticMeshActor|GetStaticMeshComponent _asstatic_mesh_actor) "0.000000,0.000000,500.000000" "None" true)
              (Class|PrimitiveComponent|AddAngularImpulseinDegrees (Variables|/Script/Engine.StaticMeshActor|GetStaticMeshComponent _asstatic_mesh_actor) (Math|Conversions|ToVector(Float) (Math|Random|RandomFloatinRange -1.8e+02 1.8e+02)) "None" true)
              (Actor|SetLifeSpan (.HitActor (Collision|BreakHitResult _array_element)) 1e+01))
            (:CastFailed
              (bind _asbp_push_button (Utilities|Casting|CastToBP_PushButton (.HitActor (Collision|BreakHitResult _array_element))))
              (Physics|SetSimulatePhysics (Variables|/Game/Assets/EOL_Content/Blueprints/BP_PushButton.BP_PushButton_C|GetButton_Frame _asbp_push_button) true)
              (Class|PrimitiveComponent|WakeRigidBody (Variables|/Game/Assets/EOL_Content/Blueprints/BP_PushButton.BP_PushButton_C|GetButton_Frame _asbp_push_button) "None")))))))
  (Class|RadialForceComponent|FireImpulse (Variables|Default|GetRadialForce)))

(event EventBeginPlay)

(event Collision|EventActorBeginOverlap
  (params (OtherActor :type Actor%20Object%20Reference)))

(event EventTick
  (params (DeltaSeconds :type Float%20%28single-precision%29)))

(fn ConstructionScript)